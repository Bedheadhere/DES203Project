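; SpawnPoint is a one-time checkpoint that updates where the player character respawns.
; When a ThirdPersonCharacter_Final first overlaps its Box, it copies the Cylinder's world transform into that character's RespawnLocation.
; It then plays a key jingle at the Cylinder and sets a Used flag so later overlaps do nothing.
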(event `self.Box.OnComponentBeginOverlap`
  (params (OverlappedComponent :type "PrimitiveComponent Object Reference") (OtherActor :type "Actor Object Reference") (OtherComp :type "PrimitiveComponent Object Reference") (OtherBodyIndex :type Integer) (bFromSweep :type Boolean) (SweepResult :type "HitResult Structure (by ref)"))
  (if (and (== (`GameplayStatics.GetObjectClass` OtherActor) "/Game/ThirdPersonBP/Blueprints/ThirdPersonCharacter_Final.ThirdPersonCharacter_Final_C") (not (`self.Used`)))
    (bind _asthird_person_character_final (cast `/Game/ThirdPersonBP/Blueprints/ThirdPersonCharacter_Final` OtherActor))
    (set `/Game/ThirdPersonBP/Blueprints/ThirdPersonCharacter_Final.RespawnLocation` (`SceneComponent.K2_GetComponentToWorld` (`self.Cylinder`)) _asthird_person_character_final)
    (`GameplayStatics.PlaySoundAtLocation` "/Game/Audio/KeyGetJingleShort_Cue.KeyGetJingleShort_Cue" (`SceneComponent.K2_GetComponentLocation` (`self.Cylinder`)) (struct) 1.0 1.0 0.0 null null null)
    (set `self.Used` true)))

(fn `UserConstructionScript`)