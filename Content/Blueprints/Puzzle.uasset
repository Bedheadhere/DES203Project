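; Pressure plate puzzle Blueprint that sinks when the player character or a PickUp object stands on it and rises when cleared.
; Box overlaps keep a count of things on the plate, with ON and Moving flags guarding each transition.
; MoveComponentTo eases the mesh 50 units down or up, using world location as the relative target.
; PlateDown and PlateUp calls follow each move to signal the change.
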(event `self.Box.OnComponentBeginOverlap`
  (params (OverlappedComponent :type "PrimitiveComponent Object Reference") (OtherActor :type "Actor Object Reference") (OtherComp :type "PrimitiveComponent Object Reference") (OtherBodyIndex :type Integer) (bFromSweep :type Boolean) (SweepResult :type "HitResult Structure (by ref)"))
  (bind _returnvalue (`GameplayStatics.GetObjectClass` OtherActor))
  (bind _thingsonplate (`self.ThingsOnPlate`))
  (bind _staticmesh (`self.StaticMesh`))
  (if (or (== _returnvalue "/Game/ThirdPersonBP/Blueprints/ThirdPersonCharacter_Final.ThirdPersonCharacter_Final_C") (== _returnvalue "/Game/Blueprints/PickUp.PickUp_C"))
    (`/Engine/EditorBlueprintResources/StandardMacros.IncrementInt` _thingsonplate
      (:`  `
        (if (and (> _thingsonplate 0) (not (`self.ON`)) (not (`self.Moving?`)))
          (set `self.Moving?` true)
          (`KismetSystemLibrary.MoveComponentTo` _staticmesh (`KismetMathLibrary.MakeVector` (.x (`SceneComponent.K2_GetComponentLocation` _staticmesh)) (.y (`SceneComponent.K2_GetComponentLocation` _staticmesh)) (+ (.z (`SceneComponent.K2_GetComponentLocation` _staticmesh)) -50.0)) (struct) true true 0.2)
          (set `self.ON` true)
          (set `self.Moving?` false)
          (`self.PlateDown`))))))

(event `self.Box.OnComponentEndOverlap`
  (params (OverlappedComponent :type "PrimitiveComponent Object Reference") (OtherActor :type "Actor Object Reference") (OtherComp :type "PrimitiveComponent Object Reference") (OtherBodyIndex :type Integer))
  (bind _returnvalue (`GameplayStatics.GetObjectClass` OtherActor))
  (bind _thingsonplate (`self.ThingsOnPlate`))
  (bind _staticmesh (`self.StaticMesh`))
  (if (or (== _returnvalue "/Game/ThirdPersonBP/Blueprints/ThirdPersonCharacter_Final.ThirdPersonCharacter_Final_C") (== _returnvalue "/Game/Blueprints/PickUp.PickUp_C"))
    (`/Engine/EditorBlueprintResources/StandardMacros.DecrementInt` _thingsonplate
      (:`  `
        (if (and (<= _thingsonplate 0) (`self.ON`) (not (`self.Moving?`)))
          (set `self.Moving?` true)
          (`KismetSystemLibrary.MoveComponentTo` _staticmesh (`KismetMathLibrary.MakeVector` (.x (`SceneComponent.K2_GetComponentLocation` _staticmesh)) (.y (`SceneComponent.K2_GetComponentLocation` _staticmesh)) (+ (.z (`SceneComponent.K2_GetComponentLocation` _staticmesh)) 50.0)) (struct) true true)
          (set `self.ON` false)
          (set `self.Moving?` false)
          (`self.PlateUp`))))))

(fn `UserConstructionScript`)