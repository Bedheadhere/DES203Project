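; Swinging axe trap that respawns the third-person player character on contact.
; On BeginPlay a timeline pitches the Rotator component back and forth from its curve, keeping the starting roll and yaw.
; A looping timer plays a quiet swing sound at the axe's location, timed separately from the animation.
; The Box overlap checks for the exact player character class before calling Respawn.
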(event `PlaySound`
  (`GameplayStatics.PlaySoundAtLocation` "/Game/Audio/Axe_SwingV2_Cue.Axe_SwingV2_Cue" (`SceneComponent.K2_GetComponentLocation` (`self.Axe_Trap_Low`)) (struct) 0.1 1.0 0.0 null null null))

(event `self.ReceiveBeginPlay`
  (set `self.InitialX` (.roll (`SceneComponent.K2_GetComponentRotation` (`self.Rotator`))))
  (set `self.InitialZ` (.yaw (`SceneComponent.K2_GetComponentRotation` (`self.Rotator`))))
  (`KismetSystemLibrary.K2_SetTimerDelegate` (delegate `PlaySound`) 1.5 true 0.5)
  (bind (_direction _axeswing) (`Timeline|Timeline_0`)
    (:`Update`
      (`SceneComponent.K2_SetWorldRotation` (`self.Rotator`) (`KismetMathLibrary.MakeRotator` (`self.InitialX`) (* _axeswing 35.0) (`self.InitialZ`)) false false))))

(event `self.Box.OnComponentBeginOverlap`
  (params (OverlappedComponent :type "PrimitiveComponent Object Reference") (OtherActor :type "Actor Object Reference") (OtherComp :type "PrimitiveComponent Object Reference") (OtherBodyIndex :type Integer) (bFromSweep :type Boolean) (SweepResult :type "HitResult Structure (by ref)"))
  (if (== (`GameplayStatics.GetObjectClass` OtherActor) "/Game/ThirdPersonBP/Blueprints/ThirdPersonCharacter_Final.ThirdPersonCharacter_Final_C")
    (bind _asthird_person_character_2 (cast `/Game/ThirdPersonBP/Blueprints/ThirdPersonCharacter_Final` OtherActor))
    (`/Game/ThirdPersonBP/Blueprints/ThirdPersonCharacter_Final.Respawn` _asthird_person_character_2)))

(fn `UserConstructionScript`)